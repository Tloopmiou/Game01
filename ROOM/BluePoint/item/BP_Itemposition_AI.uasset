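; BP_Itemposition_AI is an item spawn point actor that places and clears random items at three fixed positions.
; BeginPlay caches the world transforms of components 1, 2 and 3.
; PushItem spawns a random class from Items at each cached transform, with repeats possible, and records the spawned actors.
; ClearItem destroys the recorded actors that are still valid and empties the list.
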(event EventBeginPlay
  (Utilities|Array|Add (Variables|Default|GetPositon) (Transformation|GetWorldTransform (Variables|Default|Get1)))
  (Utilities|Array|Add (Variables|Default|GetPositon) (Transformation|GetWorldTransform (Variables|Default|Get2)))
  (Utilities|Array|Add (Variables|Default|GetPositon) (Transformation|GetWorldTransform (Variables|Default|Get3))))

(fn ConstructionScript)

(fn PushItem
  (for _index (range 0 2)
    (bind _returnvalue (Game|SpawnActorfromClass (.OutItem (Utilities|Array|Random (Variables|Default|GetItems))) (Utilities|Array|Get(acopy) (Variables|Default|GetPositon) _index) "Undefined" "MultiplyWithRoot" 0 0))
    (bind _output_get (Variables|Default|Setitem _returnvalue))
    (Utilities|Array|Add (Variables|Default|Getitemarray) _output_get)))

(fn ClearItem
  (for _array_element (Variables|Default|Getitemarray)
    (Utilities|IsValid _array_element
      (:Is%20Valid
        (Actor|DestroyActor _array_element))))
  (Utilities|Array|Clear (Variables|Default|Getitemarray)))