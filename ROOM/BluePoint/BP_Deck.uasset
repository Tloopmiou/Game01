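; BP_Deck is a card deck Blueprint that builds and shuffles its cards on BeginPlay when BeginGame is true.
; InitializeDeck pairs every Suitarray entry with every Valuearray entry as BPCardstruct items in Deck.
; Shuffle attempts random swaps, but re-rolls the index between read and write, so cards can be duplicated or lost.
; Unconnected test loops print deck contents for debugging.
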(event EventBeginPlay
  (if (Variables|Default|GetbeginGame)
    (Development|PrintString "游戏开始")
    (CallFunction|InitializeDeck)
    (CallFunction|Shuffle)
    (else
      (Development|PrintString "gamenotbegin"))))

(fn ConstructionScript)

(fn InitializeDeck
  (for _array_element (Variables|Default|Getsuitarray)
    (for _array_element_2 (Variables|Default|Getvaluearray)
      (Utilities|Array|Add (Variables|Default|GetDeck) (Utilities|Struct|MakeBP_Cardstruct _array_element _array_element_2)))))

(fn Shuffle
  (bind _deck (Variables|Default|GetDeck))
  (bind _deck_2 (Variables|Default|GetDeck))
  (bind _returnvalue (Utilities|Array|Length _deck))
  (bind _returnvalue_2 (- _returnvalue 1))
  (bind _returnvalue_3 (Math|Random|RandomIntegerinRange 0 _returnvalue_2))
  (for _index (range 0 _returnvalue_2)
    (Variables|Default|Setcurrentcard (Utilities|Array|Get(acopy) (Variables|Default|GetDeck) _index))
    (Variables|Default|Setrandomcard (Utilities|Array|Get(acopy) (Variables|Default|GetDeck) _returnvalue_3))
    (Utilities|Array|SetArrayElem _deck_2 _index (Variables|Default|Getrandomcard) true)
    (Utilities|Array|SetArrayElem _deck_2 _returnvalue_3 (Variables|Default|Getcurrentcard) true)))