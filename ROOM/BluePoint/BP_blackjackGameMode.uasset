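; Game mode that runs turn-based blackjack between the player and a Devil AI, each losing lives on lost rounds.
; BeginPlay caches table actors, and Getcard deals from a shared deck index into the active side's hand, capped at six cards.
; Turn changes judge busts, exact 21s and game over, while mutual stands compare totals.
; InitiOnce resets hands, totals and stand flags after each round and refreshes both sides' items.
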(event Custom|Gameover
  (if (<= (Variables|/Game/ROOM/BluePoint/BP_Roomhuman.BP_Roomhuman_C|Gethealthpoint (Variables|Default|GetAs%20BP%20Roomhuman)) 0)
    (Default|CallAIwin)
    (elif (<= (Variables|/Game/ROOM/BluePoint/AI/devile/BP_Devil.BP_Devil_C|GetAIchance (Variables|Default|GetBP_Devle)) 0)
      (Default|CallPlayerwin))))

(event Custom|afters
  (|aftersss))

(event Custom|Rulejudge
  (|rg))

(event EventBeginPlay
  (bind _returnvalue (Actor|GetActorOfClass "/Game/ROOM/BluePoint/BP_Deck.BP_Deck_C"))
  (Variables|Default|Setdeck _returnvalue)
  (bind _returnvalue_2 (Actor|GetActorOfClass "/Game/ROOM/BluePoint/BP_PlayerHandcards.BP_PlayerHandcards_C"))
  (Variables|Default|SetPlayerHcards _returnvalue_2)
  (bind _returnvalue_3 (Actor|GetActorOfClass "/Game/ROOM/BluePoint/BP_cardposiotion.BP_cardposiotion_C"))
  (Variables|Default|Setcardtable _returnvalue_3)
  (bind _asbp_roomhuman (Utilities|Casting|CastToBP_Roomhuman (Game|GetPlayerCharacter 0)))
  (Variables|Default|SetAs%20BP%20Roomhuman _asbp_roomhuman)
  (bind _returnvalue_4 (Actor|GetActorOfClass "/Game/ROOM/BluePoint/AI/devile/BP_Devil.BP_Devil_C"))
  (Variables|Default|SetBP_Devle _returnvalue_4)
  (bind _returnvalue_5 (Actor|GetActorOfClass "/Game/ROOM/BluePoint/item/BP_Itemposition.BP_Itemposition_C"))
  (Variables|Default|SetItem _returnvalue_5)
  (bind _returnvalue_6 (Actor|GetActorOfClass "/Game/ROOM/BluePoint/item/BP_Itemposition_AI.BP_Itemposition_AI_C"))
  (Variables|Default|SetAIitem _returnvalue_6))

(fn ConstructionScript)

(fn Getcard
  (if (Variables|Default|Getisplayer)
    ;[1 1 1] 玩家回合获取卡牌
    (if (>= (Utilities|Array|Length (Variables|/Game/ROOM/BluePoint/BP_PlayerHandcards.BP_PlayerHandcards_C|GetPHCards (Variables|Default|GetPlayerHcards))) 6)
      (Development|PrintString "卡组已满")
      (else
        (bind _returnvalue (Game|SpawnActorfromClass "/Game/ROOM/HG_Playing_Cards/Blueprints/BP_Playing_Card.BP_Playing_Card_C" (Math|Transform|MakeTransform (.location (Utilities|Array|Get(acopy) (Variables|/Game/ROOM/BluePoint/BP_cardposiotion.BP_cardposiotion_C|Getplayercardpotransform (Variables|Default|Getcardtable)) (Variables|Default|Getplayercardtag))) (.rotation (Utilities|Array|Get(acopy) (Variables|/Game/ROOM/BluePoint/BP_cardposiotion.BP_cardposiotion_C|Getplayercardpotransform (Variables|Default|Getcardtable)) (Variables|Default|Getplayercardtag))) "1.000000,1.000000,1.000000") "AlwaysSpawn" "MultiplyWithRoot" 0 0))
        (bind _output_get (Variables|Default|SetGPCard _returnvalue))
        (Default|SetCardValue _output_get "NewEnumerator0" (.suit (Utilities|Array|Get(acopy) (Variables|/Game/ROOM/BluePoint/BP_Deck.BP_Deck_C|GetDeck (Variables|Default|Getdeck)) (Variables|Default|Getcurrnttarget))) (.value (Utilities|Array|Get(acopy) (Variables|/Game/ROOM/BluePoint/BP_Deck.BP_Deck_C|GetDeck (Variables|Default|Getdeck)) (Variables|Default|Getcurrnttarget))) "NewEnumerator1")
        (Default|Rotate _output_get)
        (Utilities|Array|Add (Variables|/Game/ROOM/BluePoint/BP_PlayerHandcards.BP_PlayerHandcards_C|GetPHCards (Variables|Default|GetPlayerHcards)) (Variables|Default|GetGPCard))
        (bind _output_get_2 (Variables|Default|SetGPlayercardpoint (Math|Conversions|ToInteger(Byte) (Utilities|String|EnumtoString (.value (Utilities|Array|Get(acopy) (Variables|/Game/ROOM/BluePoint/BP_Deck.BP_Deck_C|GetDeck (Variables|Default|Getdeck)) (Variables|Default|Getcurrnttarget)))))))
        (Utilities|Array|Add (Variables|/Game/ROOM/BluePoint/BP_PlayerHandcards.BP_PlayerHandcards_C|GetPointArray (Variables|Default|GetPlayerHcards)) _output_get_2)
        (bind _result (Math|Integer|IncrementInt (Variables|Default|Getcurrnttarget))
          (:%20%20
            (Variables|Default|Setcurrnttarget _result)
            (bind _result_2 (Math|Integer|IncrementInt (Variables|Default|Getplayercardtag))
              (:%20%20
                (Variables|Default|Setplayercardtag _result_2)
                (Development|PrintString "玩家回合结束")))))))
    (else
      ;[1 1 1] 敌方回合绘制卡牌
      (Development|PrintString "敌方回合")
      (if (>= (Utilities|Array|Length (Variables|Default|GetAIhand)) 6)
        (Development|PrintString "卡组已满")
        (else
          (bind _returnvalue_2 (Game|SpawnActorfromClass "/Game/ROOM/HG_Playing_Cards/Blueprints/BP_Playing_Card.BP_Playing_Card_C" (Math|Transform|MakeTransform (.location (Utilities|Array|Get(acopy) (Variables|/Game/ROOM/BluePoint/BP_cardposiotion.BP_cardposiotion_C|GetAicardtransform (Variables|Default|Getcardtable)) (Variables|Default|Getaicardtag))) (.rotation (Utilities|Array|Get(acopy) (Variables|/Game/ROOM/BluePoint/BP_cardposiotion.BP_cardposiotion_C|GetAicardtransform (Variables|Default|Getcardtable)) (Variables|Default|Getaicardtag))) "1.000000,1.000000,1.000000") "AlwaysSpawn" "MultiplyWithRoot" 0 0))
          (Default|SetCardValue _returnvalue_2 "NewEnumerator0" (.suit (Utilities|Array|Get(acopy) (Variables|/Game/ROOM/BluePoint/BP_Deck.BP_Deck_C|GetDeck (Variables|Default|Getdeck)) (Variables|Default|Getcurrnttarget))) (.value (Utilities|Array|Get(acopy) (Variables|/Game/ROOM/BluePoint/BP_Deck.BP_Deck_C|GetDeck (Variables|Default|Getdeck)) (Variables|Default|Getcurrnttarget))) "NewEnumerator1")
          (Default|Rotate _returnvalue_2)
          (Utilities|Array|Add (Variables|Default|GetAIhand) _returnvalue_2)
          (bind _output_get_3 (Variables|Default|SetGAICardpoint (Math|Conversions|ToInteger(Byte) (Utilities|String|EnumtoString (.value (Utilities|Array|Get(acopy) (Variables|/Game/ROOM/BluePoint/BP_Deck.BP_Deck_C|GetDeck (Variables|Default|Getdeck)) (Variables|Default|Getcurrnttarget)))))))
          (Utilities|Array|Add (Variables|Default|GetGAICardnumbers) _output_get_3)
          (bind _result_3 (Math|Integer|IncrementInt (Variables|Default|Getcurrnttarget))
            (:%20%20
              (bind _output_get_4 (Variables|Default|Setcurrnttarget _result_3))
              (bind _result_4 (Math|Integer|IncrementInt (Variables|Default|Getaicardtag))
                (:%20%20
                  (Variables|Default|Setaicardtag _result_4)
                  (Development|PrintString "敌方回合结束"))))))))))

(fn Changeturn
  (if (Variables|Default|Getisplayer)
    (CallFunction|Rulejudge)
    (CallFunction|Gameover)
    ;[1 1 1] 对局中回合转换
    (Variables|Default|Setisplayer false)
    (else
      (CallFunction|Rulejudge)
      (CallFunction|Gameover)
      (Variables|Default|Setisplayer true))))

(fn CalPlayerCard
  (Default|CsumP (Variables|Default|GetPlayerHcards)))

(fn CalAICard
  (for _array_element (Variables|Default|GetGAICardnumbers)
    (Variables|Default|SetCAIarray (+ _array_element (Variables|Default|GetCAIarray))))
  (Variables|Default|SetCAISum (Variables|Default|GetCAIarray))
  (Variables|Default|SetCAIarray 0))

(fn InitiOnce
  (bind _item (Variables|Default|GetItem))
  (bind _aiitem (Variables|Default|GetAIitem))
  (Default|Initi (Variables|Default|GetPlayerHcards))
  (for _array_element (Variables|Default|GetAIhand)
    (Actor|DestroyActor _array_element))
  (Development|PrintString "开始新对局吧！" true true "(R=1.000000,G=0.194698,B=0.000000,A=1.000000)" 3e+01)
  (Variables|Default|Setplayercardtag 0)
  (Utilities|Array|Clear (Variables|Default|GetAIhand))
  (Variables|Default|SetCAISum 0)
  (Utilities|Array|Clear (Variables|Default|GetGAICardnumbers))
  (Variables|Default|Setaicardtag 0)
  (Variables|/Game/ROOM/BluePoint/BP_Roomhuman.BP_Roomhuman_C|SetStand (Variables|Default|GetAs%20BP%20Roomhuman) false)
  (Variables|/Game/ROOM/BluePoint/AI/devile/BP_Devil.BP_Devil_C|Setstandai (Variables|Default|GetBP_Devle) false)
  (Math|Integer|IncrementInt (Variables|Default|GetTurnNumber)
    (:%20%20
      (if (>= (Variables|Default|GetTurnNumber) 0)
        (if (Utilities|Array|IsNotEmpty (Variables|/Game/ROOM/BluePoint/item/BP_Itemposition.BP_Itemposition_C|Getitemarray (Variables|Default|GetItem)))
          (Default|ClearItem _item)
          (Default|PushItem _item)
          (else
            (Default|PushItem (Variables|Default|GetItem))))
        (if (Utilities|Array|IsNotEmpty (Variables|/Game/ROOM/BluePoint/item/BP_Itemposition_AI.BP_Itemposition_AI_C|Getitemarray (Variables|Default|GetAIitem)))
          (Default|ClearItem _aiitem)
          (Default|PushItem _aiitem)
          (else
            (Default|PushItem (Variables|Default|GetAIitem))))))))

(fn Standjudge
  (if (Variables|/Game/ROOM/BluePoint/BP_Roomhuman.BP_Roomhuman_C|GetStand (Variables|Default|GetAs%20BP%20Roomhuman))
    (if (Variables|/Game/ROOM/BluePoint/AI/devile/BP_Devil.BP_Devil_C|Getstandai (Variables|Default|GetBP_Devle))
      (CallFunction|Afters)
      (else
        (Variables|Default|Setisplayer false)))
    (elif (Variables|/Game/ROOM/BluePoint/AI/devile/BP_Devil.BP_Devil_C|Getstandai (Variables|Default|GetBP_Devle))
      (Variables|Default|Setisplayer true))))