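; BP_PlayerHandcards manages the player's hand in the blackjack game, holding card actors and a parallel array of their point values.
; CsumP totals the points into PCsum, and Initi destroys the cards and clears the hand.
; DeleteCard removes a card and its points by index, then re-sums and re-lays out the hand.
; Setarray snaps cards to Cardposition transforms, rotates them and writes the card count to the game mode.
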(fn ConstructionScript)

(fn CsumP
  (for _array_element (Variables|Default|GetPointArray)
    (Variables|Default|SetCPlayer%20Array (+ _array_element (Variables|Default|GetCPlayer%20Array))))
  (bind _output_get (Variables|Default|SetP_Csum (Variables|Default|GetCPlayer%20Array)))
  (Variables|Default|SetCPlayer%20Array 0)
  (Development|PrintString (Utilities|String|Append "--------------SUM:" (Utilities|String|ToString(Integer) _output_get))))

(fn Initi
  (for _array_element (Variables|Default|GetPHCards)
    (Actor|DestroyActor _array_element))
  (Utilities|Array|Clear (Variables|Default|GetPHCards))
  (Variables|Default|SetP_Csum 0)
  (Utilities|Array|Clear (Variables|Default|GetPointArray)))

(fn DeleteCard
  (params (SelectedCard :type BP%20Playing%20Card%20Object%20Reference))
  (bind _phcards (Variables|Default|GetPHCards))
  (bind _output_get (LocalVariables|Setindex (Utilities|Array|FindItem _phcards SelectedCard)))
  (if (>= _output_get 0)
    (Actor|DestroyActor (Utilities|Array|Get(acopy) _phcards _output_get))
    (Utilities|Array|RemoveItem _phcards (Utilities|Array|Get(acopy) _phcards _output_get))
    (Development|PrintString (Utilities|String|Append "Removing Index::" (Utilities|String|ToString(Integer) _output_get)))
    (Utilities|Array|RemoveIndex (Variables|Default|GetPointArray) _output_get)
    (CallFunction|CsumP)
    (CallFunction|Setarray)))

(fn Setarray
  (bind _phcards (Variables|Default|GetPHCards))
  (for (_array_element _array_index) _phcards
    (Utilities|IsValid _array_element
      (:Is%20Valid
        (Transformation|SetActorTransform _array_element (Utilities|Array|Get(acopy) (Variables|/Game/ROOM/BluePoint/BP_cardposiotion.BP_cardposiotion_C|Getplayercardpotransform (Variables|Default|Getcardposition)) _array_index))
        (Default|Rotate _array_element)
        (bind _asbp_blackjack_game_mode (Utilities|Casting|CastToBP_blackjackGameMode (Game|GetGameMode)))
        (Variables|/Game/ROOM/BluePoint/BP_blackjackGameMode.BP_blackjackGameMode_C|Setplayercardtag _asbp_blackjack_game_mode (Utilities|Array|Length _phcards))))))