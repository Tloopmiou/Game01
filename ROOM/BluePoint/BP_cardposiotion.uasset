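; BP_cardposiotion is an actor that marks the card slot positions for a card game between the player and an AI.
; On BeginPlay it fills two transform arrays from the world transforms of its card components, six slots for the player and six for the AI.
; The file only records these layouts and contains no logic that places or moves cards.
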(event EventBeginPlay
  ;[1 1 1] addplayercardposition
  (Utilities|Array|Add (Variables|Default|Getplayercardpotransform) (Transformation|GetWorldTransform (Variables|Default|GetPlayercard1)))
  (Utilities|Array|Add (Variables|Default|Getplayercardpotransform) (Transformation|GetWorldTransform (Variables|Default|GetPlayercard2)))
  (Utilities|Array|Add (Variables|Default|Getplayercardpotransform) (Transformation|GetWorldTransform (Variables|Default|GetPlayercard3)))
  (Utilities|Array|Add (Variables|Default|Getplayercardpotransform) (Transformation|GetWorldTransform (Variables|Default|GetPlayercard4)))
  (Utilities|Array|Add (Variables|Default|Getplayercardpotransform) (Transformation|GetWorldTransform (Variables|Default|GetPlayercard5)))
  (Utilities|Array|Add (Variables|Default|Getplayercardpotransform) (Transformation|GetWorldTransform (Variables|Default|GetPlayercard6)))
  ;[1 1 1] aicardposition
  (Utilities|Array|Add (Variables|Default|GetAicardtransform) (Transformation|GetWorldTransform (Variables|Default|GetAIcard1)))
  (Utilities|Array|Add (Variables|Default|GetAicardtransform) (Transformation|GetWorldTransform (Variables|Default|GetAIcard2)))
  (Utilities|Array|Add (Variables|Default|GetAicardtransform) (Transformation|GetWorldTransform (Variables|Default|GetAIcard3)))
  (Utilities|Array|Add (Variables|Default|GetAicardtransform) (Transformation|GetWorldTransform (Variables|Default|GetAIcard4)))
  (Utilities|Array|Add (Variables|Default|GetAicardtransform) (Transformation|GetWorldTransform (Variables|Default|GetAIcard5)))
  (Utilities|Array|Add (Variables|Default|GetAicardtransform) (Transformation|GetWorldTransform (Variables|Default|GetAIcard6))))

(fn ConstructionScript)