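; Card table Blueprint that provides the placement positions for player and AI cards.
; Its Construction Script reads the world transforms of six player marker components and six AI marker components.
; It appends them in a fixed order to two arrays, Playert for the player and Ait for the AI, with the player markers added in descending name order and ending on Player11.
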(fn ConstructionScript
  ;[1 1 1] addplayercardposition
  (Utilities|Array|Add (Variables|Default|Getplayert) (Transformation|GetWorldTransform (Variables|Default|Getplayer6)))
  (Utilities|Array|Add (Variables|Default|Getplayert) (Transformation|GetWorldTransform (Variables|Default|Getplayer5)))
  (Utilities|Array|Add (Variables|Default|Getplayert) (Transformation|GetWorldTransform (Variables|Default|Getplayer4)))
  (Utilities|Array|Add (Variables|Default|Getplayert) (Transformation|GetWorldTransform (Variables|Default|Getplayer3)))
  (Utilities|Array|Add (Variables|Default|Getplayert) (Transformation|GetWorldTransform (Variables|Default|Getplayer2)))
  (Utilities|Array|Add (Variables|Default|Getplayert) (Transformation|GetWorldTransform (Variables|Default|Getplayer11)))
  ;[1 1 1] aicardposition
  (Utilities|Array|Add (Variables|Default|Getait) (Transformation|GetWorldTransform (Variables|Default|Getai1)))
  (Utilities|Array|Add (Variables|Default|Getait) (Transformation|GetWorldTransform (Variables|Default|Getai2)))
  (Utilities|Array|Add (Variables|Default|Getait) (Transformation|GetWorldTransform (Variables|Default|Getai3)))
  (Utilities|Array|Add (Variables|Default|Getait) (Transformation|GetWorldTransform (Variables|Default|Getai4)))
  (Utilities|Array|Add (Variables|Default|Getait) (Transformation|GetWorldTransform (Variables|Default|Getai5)))
  (Utilities|Array|Add (Variables|Default|Getait) (Transformation|GetWorldTransform (Variables|Default|Getai6))))